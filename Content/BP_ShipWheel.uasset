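; BP_ShipWheel is a possessable ship's wheel that responds to look and move input while possessed.
; Look input pans CameraPivot within clamped yaw and pitch limits, while horizontal move input rolls WheelPivot at a frame-rate-independent speed, tracking WheelTurnAmount within a symmetric maximum.
; It exposes possession and exit point transforms; possess and release events only print debug messages, and the file applies no steering to a ship.
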(event EventBeginPlay)

(event Collision|EventActorBeginOverlap
  (params (OtherActor :type Actor%20Object%20Reference)))

(event EventTick
  (params (DeltaSeconds :type Float%20%28single-precision%29)))

(event EventPossessObject
  (params (PossessingGhost :type Actor%20Object%20Reference))
  (Development|PrintString "POSSESSED"))

(event EventStopPossessing
  (Development|PrintString "Stopped Possessing"))

(event EventPossessionLook
  (params (LookInput :type Vector%202D%20Structure))
  (Variables|Default|SetCameraYaw (Math|Float|Clamp(Float) (+ (* (.x LookInput) (Variables|Default|GetCameraPanSpeed)) (Variables|Default|GetCameraYaw)) (Variables|Default|GetMinCameraYaw) (Variables|Default|GetMaxCameraYaw)))
  (Variables|Default|SetCameraPitch (Math|Float|Clamp(Float) (+ (* (.y LookInput) (Variables|Default|GetCameraPanSpeed)) (Variables|Default|GetCameraPitch)) (Variables|Default|GetMinCameraPitch) (Variables|Default|GetMaxCameraPitch)))
  (Transformation|SetRelativeRotation (Variables|Default|GetCameraPivot) (Math|Rotator|MakeRotator 0.0 (Variables|Default|GetCameraPitch) (Variables|Default|GetCameraYaw)) false false))

(event EventPossessionMove
  (params (MoveInput :type Vector%202D%20Structure))
  (bind _output_get (Variables|Default|SetNewWheelTurnAmount (Math|Float|Clamp(Float) (+ (* (* (* (.X (Math|Vector2D|BreakVector2D MoveInput)) -1.0) (Variables|Default|GetWheelTurnSpeed)) (Utilities|Time|GetWorldDeltaSeconds)) (Variables|Default|GetWheelTurnAmount)) (* (Variables|Default|GetMaxWheelTurn) -1.0) (Variables|Default|GetMaxWheelTurn))))
  (Variables|Default|SetRotationDelta (- _output_get (Variables|Default|GetWheelTurnAmount)))
  (Variables|Default|SetWheelTurnAmount (Variables|Default|GetNewWheelTurnAmount))
  (Transformation|AddLocalRotation (Variables|Default|GetWheelPivot) (Math|Rotator|MakeRotator (Variables|Default|GetRotationDelta) 0.0 0.0) false false))

(fn ConstructionScript)

(fn GetExitTransform
  (return (Transformation|GetWorldTransform (Variables|Default|GetExitPoint))))

(fn GetPossessonTransform
  (return (Transformation|GetWorldTransform (Variables|Default|GetPossessionPoint))))