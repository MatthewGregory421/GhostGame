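; BP_Ship is a sailing ship that moves itself and carries ghost characters along with it.
; Each tick it moves forward at CurrentSpeed without sweeping and yaws by the normalized, inverted ShipWheel turn amount.
; SetSailAmount clamps sail input and instantly sets speed as a fraction of BaseSpeed.
; Ghosts attach on entering ShipInfluenceVolume, or shortly after BeginPlay if already inside, and detach on leaving, keeping world transforms.
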(event OnComponentBeginOverlap(ShipInfluenceVolume)
  (params (OverlappedComponent :type Primitive%20Component%20Object%20Reference) (OtherActor :type Actor%20Object%20Reference) (OtherComp :type Primitive%20Component%20Object%20Reference) (OtherBodyIndex :type Integer) (bFromSweep :type Boolean) (SweepResult :type Hit%20Result%20Structure%20%28by%20ref%29))
  (bind _asbp_ghost_character (Utilities|Casting|CastToBP_GhostCharacter OtherActor))
  (CallFunction|HandleGhostEnteredShip _asbp_ghost_character))

(event OnComponentEndOverlap(ShipInfluenceVolume)
  (params (OverlappedComponent :type Primitive%20Component%20Object%20Reference) (OtherActor :type Actor%20Object%20Reference) (OtherComp :type Primitive%20Component%20Object%20Reference) (OtherBodyIndex :type Integer))
  (Utilities|Casting|CastToBP_GhostCharacter OtherActor)
  (Transformation|DetachFromActor OtherActor "KeepWorld" "KeepWorld" "KeepWorld"))

(event EventTick
  (params (DeltaSeconds :type Float%20%28single-precision%29))
  (bind _shipwheel (Variables|Default|GetShipWheel))
  (Utilities|FlowControl|Sequence
    (:then_0
      (Transformation|AddActorWorldOffset (* (* (Variables|Default|GetCurrentSpeed) DeltaSeconds) (Transformation|GetActorForwardVector))))
    (:then_1
      (bind _output_get (Variables|Default|SetSteeringInput (/ (Variables|/Game/BP_ShipWheel.BP_ShipWheel_C|GetWheelTurnAmount _shipwheel) (Variables|/Game/BP_ShipWheel.BP_ShipWheel_C|GetMaxWheelTurn _shipwheel))))
      (Transformation|AddActorLocalRotation (Math|Rotator|MakeRotator 0.0 0.0 (* (* (* _output_get -1.0) (Variables|Default|GetMaxTurnSpeed)) (Utilities|Time|GetWorldDeltaSeconds))) false false))))

(event EventBeginPlay
  (Utilities|FlowControl|Delay 0.05)
  (for _array_element (Collision|GetOverlappingActors (Variables|Default|GetShipInfluenceVolume) "/Game/BP_GhostCharacter.BP_GhostCharacter_C" :!class /Script/Engine.PrimitiveComponent)
    (bind _asbp_ghost_character (Utilities|Casting|CastToBP_GhostCharacter _array_element))
    (CallFunction|HandleGhostEnteredShip _asbp_ghost_character)))

(fn ConstructionScript)

(fn HandleGhostEnteredShip
  (params (Ghost :type BP%20Ghost%20Character%20Object%20Reference))
  (Transformation|AttachActorToActor Ghost self "None" "KeepWorld" "KeepWorld" "KeepWorld" true))

(fn SetSailAmount
  (params (NewSailAmount :type Float%20%28double-precision%29))
  (bind _output_get (Variables|Default|SetSailAmount (Math|Float|Clamp(Float) NewSailAmount)))
  (bind _output_get_2 (Variables|Default|SetDesiredSpeed (* (Variables|Default|GetBaseSpeed) _output_get)))
  (Variables|Default|SetCurrentSpeed _output_get_2))