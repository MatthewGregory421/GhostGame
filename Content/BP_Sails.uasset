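; BP_Sails is a possessable sail control that lets the player adjust a ship's sail amount.
; While possessed, look input rotates a camera pivot within yaw and pitch limits, and move input raises or lowers a normalized sail amount over time.
; That amount is sent to the Ship and shown by scaling the sail mesh's Y axis from its initial scale.
; The possession point supplies the possession transform; the exit transform is unimplemented.
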(event EventPossessionMove
  (params (MoveInput :type Vector%202D%20Structure))
  (bind _output_get (Variables|Default|SetSailAmount (Math|Float|Clamp(Float) (+ (Variables|Default|GetSailAmount) (* (* (* (.y MoveInput) -1.0) (Variables|Default|GetSailAdjustSpeed)) (Utilities|Time|GetWorldDeltaSeconds))))))
  (Default|SetSailAmount (Variables|Default|GetShip) _output_get)
  (CallFunction|UpdateSailVisual))

(event EventBeginPlay
  (Variables|Default|SetSailFullScale (Variables|/Script/Engine.SceneComponent|GetRelativeScale3D (Variables|Default|GetSail%20Mesh))))

(event EventPossessionLook
  (params (LookInput :type Vector%202D%20Structure))
  ;[0.15 0.15 0.15 0.5] CameraFunctionality
  (Variables|CameraSettings|SetCameraYaw (Math|Float|Clamp(Float) (+ (* (.x LookInput) (Variables|CameraSettings|GetCameraPanSpeed)) (Variables|CameraSettings|GetCameraYaw)) (Variables|CameraSettings|GetMinCameraYaw) (Variables|CameraSettings|GetMaxCameraYaw)))
  (Variables|CameraSettings|SetCameraPitch (Math|Float|Clamp(Float) (+ (* (.y LookInput) (Variables|CameraSettings|GetCameraPanSpeed)) (Variables|CameraSettings|GetCameraPitch)) (Variables|CameraSettings|GetMinCameraPitch) (Variables|CameraSettings|GetMaxCameraPitch)))
  (Transformation|SetRelativeRotation (Variables|Default|GetCameraPivot) (Math|Rotator|MakeRotator 0.0 (Variables|CameraSettings|GetCameraPitch) (Variables|CameraSettings|GetCameraYaw)) false false))

(fn ConstructionScript)

(fn UpdateSailVisual
  (bind _sailfullscale (Variables|Default|GetSailFullScale))
  (Transformation|SetRelativeScale3D (Variables|Default|GetSail%20Mesh) (Math|Vector|MakeVector (.x _sailfullscale) (* (.y _sailfullscale) (Math|Float|Lerp 0.1 1.0 (Variables|Default|GetSailAmount))) (.z _sailfullscale))))

(fn GetExitTransform
  (return ""))

(fn GetPossessonTransform
  (return (Transformation|GetWorldTransform (Variables|Default|GetPossessiongPoint))))