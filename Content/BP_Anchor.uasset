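; BP_Anchor is a possessable ship anchor station that lets the player raise or drop the anchor.
; Look input turns a camera pivot within clamped yaw and pitch limits.
; Vertical move input past a threshold notifies the Ship of the anchor state and plays or reverses a timeline that lerps the mesh from its starting position.
; It supplies a possession transform, while GetExitTransform is unimplemented and a second drop timeline never runs.
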(event EventPossessionMove
  (params (MoveInput :type Vector%202D%20Structure))
  (bind _raisedanchorlocation (Variables|Default|GetRaisedAnchorLocation))
  (bind _ship (Variables|Default|GetShip))
  (Utilities|FlowControl|Sequence
    (:then_0
      (if (> (.y MoveInput) 0.5)
        (bind _output_get (Variables|Default|SetAnchorDropped false))
        (Default|SetAnchorDropped _ship _output_get)
        (bind _alpha (Timeline|Timeline_0 Reverse)
          (:Update
            (Transformation|SetRelativeLocation (Variables|Default|GetStaticMesh) (Math|Vector|Lerp(Vector) _raisedanchorlocation (+ _raisedanchorlocation (Math|Vector|MakeVector 0.0 0.0 (Variables|Default|GetAnchorDropDistance))) _alpha) false false)))))
    (:then_1
      (if (< (.y MoveInput) -0.5)
        (bind _output_get_2 (Variables|Default|SetAnchorDropped true))
        (Default|SetAnchorDropped _ship _output_get_2)
        (Timeline|Timeline_0 Play)))))

(event EventBeginPlay
  (Variables|Default|SetRaisedAnchorLocation (Variables|/Script/Engine.SceneComponent|GetRelativeLocation (Variables|Default|GetStaticMesh))))

(event EventPossessionLook
  (params (LookInput :type Vector%202D%20Structure))
  ;[0.15 0.15 0.15 0.5] CameraFunctionality
  (Variables|CameraSettings|SetCameraYaw (Math|Float|Clamp(Float) (+ (* (.x LookInput) (Variables|CameraSettings|GetCameraPanSpeed)) (Variables|CameraSettings|GetCameraYaw)) (Variables|CameraSettings|GetMinCameraYaw) (Variables|CameraSettings|GetMaxCameraYaw)))
  (Variables|CameraSettings|SetCameraPitch (Math|Float|Clamp(Float) (+ (* (.y LookInput) (Variables|CameraSettings|GetCameraPanSpeed)) (Variables|CameraSettings|GetCameraPitch)) (Variables|CameraSettings|GetMinCameraPitch) (Variables|CameraSettings|GetMaxCameraPitch)))
  (Transformation|SetRelativeRotation (Variables|Default|GetCameraPivot) (Math|Rotator|MakeRotator 0.0 (Variables|CameraSettings|GetCameraPitch) (Variables|CameraSettings|GetCameraYaw)) false false))

(fn ConstructionScript)

(fn GetExitTransform
  (return ""))

(fn GetPossessonTransform
  (return (Transformation|GetWorldTransform (Variables|Default|GetPossessionPoint))))